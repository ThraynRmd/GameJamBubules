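; GM_Play is a game mode that sets up local multiplayer, with one player per PlayerStart in the level.
; On BeginPlay it loops over the PlayerStarts, calls CreatePlayer with each index and prints that index.
; Each controller gets the IMP_Play Enhanced Input mapping context and possesses a BP_Player spawned at its start.
; The first index uses the existing player controller 0 instead of the CreatePlayer result.
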(event EventBeginPlay
  (bind _outactors (Actor|GetAllActorsOfClass "/Script/Engine.PlayerStart"))
  (for (_array_element _array_index) _outactors
    (bind _output_get (Variables|Default|SetArray%20Index _array_index))
    (bind _returnvalue (Class|GameplayStatics|CreatePlayer _output_get))
    (Development|PrintString (Utilities|String|ToString(Integer) _output_get))
    (if (> (Variables|Default|GetArray%20Index) 0)
      (Input|AddMappingContext (PlayerController|LocalPlayerSubsystems|GetEnhancedInputLocalPlayerSubsystem _returnvalue) "/Game/input/IMP_Play.IMP_Play" 0 "(bIgnoreAllPressedKeysUntilRelease=True,bForceImmediately=False)")
      (bind _returnvalue_2 (Game|SpawnActorfromClass "/Game/BP_Player.BP_Player_C" (Transformation|GetActorTransform _array_element) "Undefined" 0 0)) ; BP_Player
      (Pawn|Possess _returnvalue _returnvalue_2)
      (else
        (Input|AddMappingContext (PlayerController|LocalPlayerSubsystems|GetEnhancedInputLocalPlayerSubsystem (Game|GetPlayerController 0)) "/Game/input/IMP_Play.IMP_Play" 0 "(bIgnoreAllPressedKeysUntilRelease=True,bForceImmediately=False)")
        (bind _returnvalue_3 (Game|SpawnActorfromClass "/Game/BP_Player.BP_Player_C" (Transformation|GetActorTransform _array_element) "Undefined" 0 0)) ; BP_Player
        (Pawn|Possess (Game|GetPlayerController 0) _returnvalue_3)))))

(event EventTick
  (params (DeltaSeconds :type Float%20%28single-precision%29)))

(fn ConstructionScript)