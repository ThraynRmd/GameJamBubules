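; GM_PLay sets up local multiplayer at BeginPlay, with one player per placed actor of a class the graph leaves unspecified.
; Each actor index gets a CreatePlayer call, then a BP_PlayerTest spawned at that actor's transform and possessed by the matching controller.
; Index 0 uses the existing first controller for its input subsystem, while later indices use the created one.
; Mapping contexts and the player class are marked as placeholders.
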(event EventBeginPlay
  (bind _returnvalue (Game|GetPlayerController 0))
  (bind _outactors (Actor|GetAllActorsOfClass 0))
  (for (_array_element _array_index) _outactors
    (bind _output_get (Variables|Default|SetArray%20Index _array_index))
    (bind _returnvalue_2 (Class|GameplayStatics|CreatePlayer _output_get))
    (if (> (Variables|Default|GetArray%20Index) 0)
      (Input|AddMappingContext (PlayerController|LocalPlayerSubsystems|GetEnhancedInputLocalPlayerSubsystem _returnvalue_2) 0 0 "(bIgnoreAllPressedKeysUntilRelease=True,bForceImmediately=False,bNotifyUserSettings=False)") ; IMC à add
      (bind _returnvalue_3 (Game|SpawnActorfromClass "/Game/Blueprint/BP_PlayerTest.BP_PlayerTest_C" (Transformation|GetActorTransform _array_element) "Undefined" "MultiplyWithRoot" 0 0)) ; BP_Player
      (Pawn|Possess (Game|GetPlayerController (Variables|Default|GetArray%20Index)) _returnvalue_3)
      (else
        (Input|AddMappingContext (PlayerController|LocalPlayerSubsystems|GetEnhancedInputLocalPlayerSubsystem _returnvalue) 0 0 "(bIgnoreAllPressedKeysUntilRelease=True,bForceImmediately=False,bNotifyUserSettings=False)") ; IMC à add
        (bind _returnvalue_4 (Game|SpawnActorfromClass "/Game/Blueprint/BP_PlayerTest.BP_PlayerTest_C" (Transformation|GetActorTransform _array_element) "Undefined" "MultiplyWithRoot" 0 0)) ; BP Player a add
        (Pawn|Possess _returnvalue _returnvalue_4)))))

(event EventTick
  (params (DeltaSeconds :type Float%20%28single-precision%29)))

(fn ConstructionScript)