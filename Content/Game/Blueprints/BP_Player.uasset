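; Player Blueprint that receives move, dash and attack events and hands movement work to components.
; Move input drives BPCMovement's move or stop dispatchers and toggles the Run component, while Tick applies location and prints capsule velocity for debugging.
; Dash calls BPCDash's dispatcher and activates the Dash component for a short delay.
; Light and heavy attacks are placeholders that only print text.
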(event EventIMove
  (params (TargetDirection :type Vector%202D%20Structure))
  (if (Class|KismetMathLibrary|EqualExactlyVector2DVector2D TargetDirection)
    (Default|CallEDonStopMove (Variables|Default|GetBPC_Movement))
    (Components|Activation|SetActive (Variables|Default|GetRun) false false)
    (else
      (Default|CallEDonMove (Variables|Default|GetBPC_Movement) TargetDirection)
      (Components|Activation|SetActive (Variables|Default|GetRun) true false))))

(event EventTick
  (params (DeltaSeconds :type Float%20%28single-precision%29))
  (Default|ApplyLocation (Variables|Default|GetBPC_Movement))
  (Development|PrintText (Utilities|Text|FormatText "Velocity {x}" (Utilities|String|ToString(Vector) (Transformation|GetComponentVelocity (Variables|Collision|GetCapsuleComponent)))) true true "(R=0.000000,G=0.660000,B=1.000000,A=1.000000)" 0.0))

(event EventIAttackLight
  (Development|PrintText "Light Attack"))

(event EventIHeavyAttack
  (params (PowerRatio :type Float%20%28double-precision%29))
  (Development|PrintText "Heavy Attack"))

(event EventIDash
  (Components|Activation|SetActive (Variables|Default|GetDash) true true)
  (Development|PrintText "Dash")
  (Default|CallEDonDash (Variables|Default|GetBPC_Dash))
  (Utilities|FlowControl|Delay 0.5)
  (Components|Activation|SetActive (Variables|Default|GetDash) false false))

(event EventBeginPlay)

(fn ConstructionScript)