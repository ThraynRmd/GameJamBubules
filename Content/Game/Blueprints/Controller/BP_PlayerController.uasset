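; BP_PlayerController is a player controller that turns Enhanced Input actions into commands for the player character.
; Move, dash, light attack and heavy attack actions each send an interface message to the character found through this controller's ID, so no cast is needed.
; Move forwards its action value on both trigger and completion, and heavy attack passes along its elapsed time.
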(event Input|EnhancedActionEvents|EnhancedInputActionIA_LightAttack
  (params (ActionValue :type Boolean) (ElapsedSeconds :type Float%20%28double-precision%29) (TriggeredSeconds :type Float%20%28double-precision%29) (InputAction :type Input%20Action%20Object%20Reference :default "/Game/Game/Input/Actions/IA_LightAttack.IA_LightAttack"))
  (:Triggered
    (Class|BPIAttack|IAttackLight(Message) (Game|GetPlayerCharacter (Class|GameplayStatics|GetPlayerControllerID self)))))

(event Input|EnhancedActionEvents|EnhancedInputActionIA_Move
  (params (ActionValue :type Vector%202D%20Structure) (ElapsedSeconds :type Float%20%28double-precision%29) (TriggeredSeconds :type Float%20%28double-precision%29) (InputAction :type Input%20Action%20Object%20Reference :default "/Game/Game/Input/Actions/IA_Move.IA_Move"))
  (:Triggered
    (Class|BPIMovement|IMove(Message) (Game|GetPlayerCharacter (Class|GameplayStatics|GetPlayerControllerID self)) ActionValue :!label _label))
  (:Completed
    (goto _label)))

(event Input|EnhancedActionEvents|EnhancedInputActionIA_HeavyAttack
  (params (ActionValue :type Boolean) (ElapsedSeconds :type Float%20%28double-precision%29) (TriggeredSeconds :type Float%20%28double-precision%29) (InputAction :type Input%20Action%20Object%20Reference :default "/Game/Game/Input/Actions/IA_HeavyAttack.IA_HeavyAttack"))
  (:Triggered
    (Class|BPIAttack|IHeavyAttack(Message) (Game|GetPlayerCharacter (Class|GameplayStatics|GetPlayerControllerID self)) ElapsedSeconds)))

(event Input|EnhancedActionEvents|EnhancedInputActionIA_Dash
  (params (ActionValue :type Boolean) (ElapsedSeconds :type Float%20%28double-precision%29) (TriggeredSeconds :type Float%20%28double-precision%29) (InputAction :type Input%20Action%20Object%20Reference :default "/Game/Game/Input/Actions/IA_Dash.IA_Dash"))
  (:Triggered
    (Class|BPIMovement|IDash(Message) (Game|GetPlayerCharacter (Class|GameplayStatics|GetPlayerControllerID self)))))

(fn ConstructionScript)