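; BP_GameMode runs a local multiplayer last-player-standing match with periodic boost pickups.
; On BeginPlay it creates a local player for each PlayerStart, spawns and possesses a BP_Player, then triggers a camera update.
; Destroyed players leave the tracked array; when one or none remains, the win widget appears, and GiveWinPlayer exposes the first remaining player's controller.
; A looping timer spawns BP_Boost at random TargetPoints.
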(event Custom|Player_ED_PlayerDestroyed_Event
  (params (PlayerDeath :type BP%20Player%20Object%20Reference))
  (bind _player (Variables|Default|GetPlayer))
  (Utilities|Array|RemoveItem _player PlayerDeath)
  (Development|PrintString "Hello")
  (if (<= (Utilities|Array|Length _player) 1)
    (bind _returnvalue (UserInterface|CreateWidget "/Game/Game/Blueprints/Widgets/UW_MainWin.UW_MainWin_C"))
    (UserInterface|Viewport|AddtoPlayerScreen _returnvalue)))

(event Custom|Spawn%20Bonus
  (Game|SpawnActorfromClass "/Game/Game/Blueprints/Boost/BP_Boost.BP_Boost_C" (Transformation|GetActorTransform (.OutItem (Utilities|Array|Random (Variables|Default|GetSpawn%20Bonus%20Location)))) "AdjustIfPossibleButAlwaysSpawn" 0 0))

(event Custom|StartSpawnBoost
  (Utilities|Time|SetTimerbyEvent (delegate Custom|Spawn%20Bonus) 5.0 true))

(event EventBeginPlay
  ;[1 0.0371 0] AAAAAAAAAAAAAAAAAAAAAAAAAAAAAAAAAAAAAAAAAAAAAAAAAAAAAAAAAAAAAAAAAAAAAAAAAAAAAAAAAAAAAAAAAAAAAAAAAAAAAAAAAAAAAAAAAAAAAAAAAAAAAAAAAAAAAAAAAAAAAAAAAAAAAAAAAAAAAAAAAAAAAAAAAAAAAAAAAAAAAAAAAAAAAAAAAAAAAAAAAAAAAAAAAAAAAAAAAAAAAAAAAAAAAAAAAAAAAAAAAAAAAAAAAAAAAAAAAAAAAAAAAAAAAAAAAAAAAAAAAAAAAAAAAAAAAAAAAAAAAAAAAAAAAAAAAAAAAAAAAAAAAAAAAAAAAAAAAAAAAAAAAAAAAAAAAAAAAAAAAAAAAAAAAAAAAAAAAAAAAAAAAAAAAAAAAAAAAAAAAAAAAAAAAAAAAAAAAAAAAAAAAAAAAAAAAAAAAAAAAAAAAAAAAAAAAAAAAAAAAAAAAAAAAAAAAAAAAAAAAAAAAAAAAAAAAAAAAAAAAAAAAAAAAAAAAAAAAAAAAAAAAAAAAAAAAAAAAAAAAAAAAAAAAAAAAAAAAAAAAAAAAAAAAAAAAAAAAAAAAAAAAAAAAAAAAAAAAAAAAAAAAAAAAAAAAAAAAAAAAAAAAAAAAAAAAAAAAAAAAAAAAAAAAAAAAAAAAAAAAAAAAAAAAAAAAAAAAAAAAAAAAAAAAAAAAAAAAAAAAAAAAAAAAAAAAAAAAAAAAAAAAAAAAAAAAAAAAAAAAAAAAAAAAAAAAAAAAAAAAAAAAAAAAAAAAAAAAAAAAAAAAAAAAAAAAAAAAAAAAAAAAAAAAAAAAAAAAAAAAAAAAAAAAAAAAAAAAAAAAAAAAAAAAAAAAAAAAAAAAAAAAAAAAAAAAAAAAAAAAAAAAAAAAAAAAAAAAAAAAAAAAAAAAAAAAAAAAAAAAAAAAAAAAAAAAAAAAAAAAAAAAAAAAAAAAAAAAAAAAAAAAAAAAAAAAAAAAAAAAAAAAAAAAAAAAAAAAAAAAAAAAAAAAAAAAAAAAAAAAAAAAAAAAAAAAAAAAAAAAAAAAAAAAAAAAAAAAAAAAAAAAAAAAAAAAAAAAAAAAAAAAAAAAAAAAAAAAAAAAAAAAAAAAAAAAAAAAAAAAAAAAAAAAAAAAAAAAAAAAAAAAAAAAAAAAAAAAAAAAAAAAAAAAAAAAAAAAAAAAAAAAAAAAAAAAAAAAAAAAAAAAAAAAAAAAAAAAAAAAAAAAAAAAAAAAAAAAAAAAAAAAAAAAAAAAAAAAAAAAAAAAAAAAAAAAAAAAAAAAAAAAAAAAAAAAAAAAAAAAAAAAAAAAAAAAAAAAAAAAAAAAAAAAAAAAAAAAAAAAAAAAAAAAAAAAAAAAAAAAAAAAAAAAAAAAAAAAAAAAAAAAAAAAAAAAAAAAAAAAAAAAAAAAAAAAAAAAAAAAAAAAAAAAAAAAAAAAAAAAAAAAAAAAAAAAAAAAAAAAAAAAAAAAAAAAAAAAAAAAAAAAAAAAAAAAAAAAAAAAAAAAAAAAAAAAAAAAAAAAAAAAAAAAAAAAAAAAAAAAAAAAAAAAAAAAAAAAAAAAAAAAAAAAAAAAAAAAAAAAAAAAAAAAAAAAAAAAAAAAAAAAAAAAAAAAAAAAAAAAAAAAAAAAAAAAAAAAAAAAAAAAAAAAAAAAAAAAAAAAAAAAAAAAAAAAAAAAAAAAAAAAAAAAAAAAAAAAAAAAAAAAAAAAAAAAAAAAAAAAAAAAAAAAAAAAAAAAAAAAAAAAAAAAAAAAAAAAAAAAAAAAAAAAAAAAAAAAAAAAAAAAAAAAAAAAAAAAAAAAAAAAAAAAAAAAAAAAAAAAAAAAAAAAAAAAAAAAAAAAAAAAAAAAAAAAAAAAAAAAAAAAAAAAAAAAAAAAAAAAAAAAAAAAAAAAAAAAAAAAAAAAAAAAAAAAAAAAAAAAAAAAAAAAAAAAAAAAAAAAAAAAAAAAAAAAAAAAAAAAAAAAAAAAAAAAAAAAAAAAAAAAAAAAAAAAAAAAAAAAAAAAAAAAAAAAAAAAAAAAAAAAAAAAAAAAAAAAAAAAAAAAAAAAAAAAAAAAAAAAAAAAAAAAAAAAAAAAAAAAAAAAAAAAAAAAAAAAAAAAAAAAAAAAAAAAAAAAAAAAAAAAAAAAAAAAAAAAAAAAAAAAAAAAAAAAAAAAAAAAAAAAAAAAAAAAAAAAAAAAAAAAAAAAAAAAAAAAAAAAAAAAAAAAAAAAAAAAAAAAAAAAAAAAAAAAAAAAAAAAAAAAAAAAAAAAAAAAAAAAAAAAAAAAAAAAAAAAAAAAAAAAAAAAAAAAAAAAAAAAAAAAAAAAAH  (Aussi long que les 7h que j'ai passé à faire marcher cte merde ^-^)
  (CallFunction|PlayerCreation)
  (Default|CallCameraUpdate)
  (bind _outactors (Actor|GetAllActorsOfClass "/Game/Game/Blueprints/BP_Player.BP_Player_C"))
  (Variables|Default|SetPlayer _outactors)
  (bind _outactors_2 (Actor|GetAllActorsOfClass "/Script/Engine.TargetPoint"))
  (Variables|Default|SetSpawn%20Bonus%20Location _outactors_2)
  (CallFunction|StartSpawnBoost))

(fn ConstructionScript)

(fn GiveWinPlayer
  (bind _player (Variables|Default|GetPlayer))
  (bind _output (Utilities|Array|Get(acopy) _player))
  (Utilities|IsValid _output
    (:Is%20Valid
      (bind _asbp_player (Utilities|Casting|CastToBP_Player _output)
        (:then
          (bind _as_bp_player_controller (Default|GetController _asbp_player))
          (return _as_bp_player_controller (Class|GameplayStatics|GetPlayerControllerID _as_bp_player_controller)))
        (:CastFailed
          (return 0 0))))
    (:Is%20Not%20Valid
      (Development|PrintString "Je suis vide"))))

(fn PlayerCreation
  (bind _outactors (Actor|GetAllActorsOfClass "/Script/Engine.PlayerStart"))
  (bind _output_get (LocalVariables|SetPlayerStart _outactors))
  (for (_ _array_index) _output_get
    (LocalVariables|SetCurrentIndex _array_index)
    (Utilities|IsValid (Class|GameplayStatics|GetPlayerControllerfromID (LocalVariables|GetCurrentIndex))
      (:Is%20Valid
        (LocalVariables|SetCurrentController (Class|GameplayStatics|GetPlayerControllerfromID (LocalVariables|GetCurrentIndex))))
      (:Is%20Not%20Valid
        (bind _returnvalue (Class|GameplayStatics|CreatePlayer (LocalVariables|GetCurrentIndex)))
        (LocalVariables|SetCurrentController _returnvalue)))
    (Input|AddMappingContext (PlayerController|LocalPlayerSubsystems|GetEnhancedInputLocalPlayerSubsystem (LocalVariables|GetCurrentController)) "/Game/Game/Input/IMC_Player.IMC_Player" 0 "(bIgnoreAllPressedKeysUntilRelease=True,bForceImmediately=False)")
    (bind _returnvalue_2 (Game|SpawnActorfromClass "/Game/Game/Blueprints/BP_Player.BP_Player_C" (Transformation|GetActorTransform (Utilities|Array|Get(acopy) (LocalVariables|GetPlayerStart) (LocalVariables|GetCurrentIndex))) "Undefined" 0 0))
    (EventDispatchers|BindEventtoEDActorDestroyed _returnvalue_2 (EventDispatchers|CreateEvent :!event Custom|Player_ED_PlayerDestroyed_Event))
    (Pawn|Possess (LocalVariables|GetCurrentController) _returnvalue_2))
  (return))