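; Blueprint function library of shared helpers for rotation alignment and countdown timing.
; AlignVector gives a scene component's current relative rotation and a look-at rotation along a goal direction, both as quaternions.
; AlignSmooth converts two quaternions to rotators and interpolates between them using world delta time.
; TimerNeg decrements a by-ref value by scaled delta time, reports expiry, then clamps to zero or resets to the maximum.
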(fn AlignSmooth
  (params (CurrentRota :type Quat%20Structure) (TargetRota :type Quat%20Structure) (InterpSpeed :type Float%20%28double-precision%29))
  (return (Math|Interpolation|RInterpTo (Class|KismetMathLibrary|QuatRotator CurrentRota) (Class|KismetMathLibrary|QuatRotator TargetRota) (Utilities|Time|GetWorldDeltaSeconds) InterpSpeed)))

(fn AlignVector
  (params (Target :type Scene%20Component%20Object%20Reference) (Goal :type Vector))
  (bind _returnvalue (Transformation|GetWorldLocation Target))
  (bind _returnvalue_2 (* Goal 5e+02))
  (bind _returnvalue_3 (+ _returnvalue _returnvalue_2))
  (bind _returnvalue_4 (Math|Rotator|FindLookatRotation _returnvalue _returnvalue_3))
  (bind _returnvalue_5 (Math|Conversions|ToQuaternion(Rotator) _returnvalue_4))
  (bind _output_get (LocalVariables|SetCurrentRotation (Math|Conversions|ToQuaternion(Rotator) (Variables|/Script/Engine.SceneComponent|GetRelativeRotation Target))))
  (LocalVariables|SetTargetRotationQuat (* _returnvalue_5 _output_get))
  (return (LocalVariables|GetCurrentRotation) _returnvalue_5))

(fn TimerNeg
  (params (Current :type Float%20%28double-precision%29%20%28by%20ref%29) (TimeMax :type Float%20%28double-precision%29) (MultiplierTime :type Float%20%28double-precision%29) (AutoReset :type Boolean))
  (LocalVariables|SetFutureTime (- Current (* (Utilities|Time|GetWorldDeltaSeconds) MultiplierTime)))
  (bind _output_get (LocalVariables|SetTimeSpended (<= (LocalVariables|GetFutureTime) 0.0)))
  (if _output_get
    (if AutoReset
      (LocalVariables|SetFutureTime TimeMax)
      (else
        (LocalVariables|SetFutureTime 0.0))))
  (|SetBy-RefVar Current (LocalVariables|GetFutureTime))
  (return (LocalVariables|GetTimeSpended)))