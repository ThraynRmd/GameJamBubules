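; BP_Boost is a pickup actor that grants the player a random boost on contact.
; On BeginPlay it picks one component class at random from its BoostClass array.
; When a BP_PlayerRefonte overlaps it, it adds that component to the player, calls its EDOnAdded event with the player, then destroys itself.
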(event EventBeginPlay
  (bind _boostclass (Variables|Default|GetBoostClass))
  (Variables|Default|SetCurrentBoost (Utilities|Array|Get(acopy) _boostclass (Math|Random|RandomIntegerinRange 0 (- (Utilities|Array|Length _boostclass) 1)))))

(event Collision|EventActorBeginOverlap
  (params (OtherActor :type Actor%20Object%20Reference))
  (bind _asbp_player_refonte (Utilities|Casting|CastToBP_PlayerRefonte OtherActor))
  (bind _returnvalue (Game|AddComponentbyClass _asbp_player_refonte (Variables|Default|GetCurrentBoost)))
  (Default|CallEDonAdded _returnvalue _asbp_player_refonte)
  (Actor|DestroyActor))

(fn ConstructionScript)