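; Player pawn built on a physics sphere, forwarding move, stop and dash interface events to movement and dash components through event dispatchers.
; On BeginPlay it caches the player controller after a short delay, then applies a random mesh and anim class from DT_Chara.
; It also derives the movement component's ground detection length from the sphere radius.
; Destruction disables input, physics and collision, then broadcasts OnDestroy without removing the actor.
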(event Custom|Destroy_Event
  (bind _sphere (Variables|Default|GetSphere))
  (Input|DisableInput (Variables|Default|GetPlayerController))
  (Physics|SetSimulatePhysics _sphere false)
  (Collision|SetCollisionEnabled _sphere "NoCollision")
  (Default|CallEDonDestroy self))

(event EventBeginPlay
  (bind _skm_skin (Variables|Default|GetSKM_Skin))
  (Utilities|FlowControl|Sequence
    (:then_0
      (Utilities|FlowControl|Delay 0.2)
      (bind _asbp_player_controller (Utilities|Casting|CastToBP_PlayerController (Pawn|GetController)))
      (Variables|Default|SetPlayerController _asbp_player_controller)
      (bind _outrownames (DataTable|GetDataTableRowNames "/Game/Game/Data/DT_Chara.DT_Chara"))
      (bind _returnvalue (Utilities|GetDataTableRow "/Game/Game/Data/DT_Chara.DT_Chara" (.OutItem (Utilities|Array|Random _outrownames)))
        (:then
          (Components|SkeletalMesh|SetSkeletalMeshAsset _skm_skin (.skm _returnvalue))
          (Class|SkeletalMeshComponent|SetAnimClass _skm_skin (.bp_anim _returnvalue)))))
    (:then_1
      (Variables|/Game/Game/Blueprints/Components/BPC_Movement.BPC_Movement_C|SetLengthDetectionGround (Variables|Default|GetBPC_Movement) (+ (Variables|/Script/Engine.SphereComponent|GetSphereRadius (Variables|Default|GetSphere)) 5e+01)))))

(event EventIMove
  (params (TargetDirection :type Vector%202D%20Structure))
  (Default|CallEDonMove (Variables|Default|GetBPC_Movement) TargetDirection))

(event EventIDash
  (Default|CallEDonDash (Variables|Default|GetBPC_Dash)))

(event EventIStopMove
  (Default|CallEDonStopMove (Variables|Default|GetBPC_Movement)))

(fn ConstructionScript)