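; BPC_Health is an actor component that tracks health, starting at MaxHealth on BeginPlay.
; ApplyDamage subtracts damage, clamping at zero; non-lethal hits call BecomeInvulnerable and enable Tick, which counts down CurrentTimeInv.
; BecomeInvulnerable is meant to broadcast state changes through become/leave dispatchers.
; ApplyDamage never checks invulnerability or fires damage/death dispatchers, their bound handlers are empty, and nothing ends invulnerability or reaches the tick-disable node.
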(event Custom|ED_OnDamaged_Event)

(event Custom|ED_OnDie_Event)

(event EventBeginPlay
  (Variables|Health|SetCurrentHealth (Variables|Health|GetMaxHealth))
  (EventDispatchers|BindEventtoEDonDamaged (EventDispatchers|CreateEvent :!event Custom|ED_OnDamaged_Event))
  (EventDispatchers|BindEventtoEDonDie (EventDispatchers|CreateEvent :!event Custom|ED_OnDie_Event)))

(event EventTick
  (params (DeltaSeconds :type Float%20%28single-precision%29))
  (Variables|Timer|SetCurrentTimeInv (- (Variables|Timer|GetCurrentTimeInv) (Utilities|Time|GetWorldDeltaSeconds))))

(fn ApplyDamage
  (params (DamageTaken :type Integer))
  (if (<= (- (Variables|Health|GetCurrentHealth) DamageTaken) 0)
    (Variables|Health|SetCurrentHealth 0)
    (else
      (Variables|Health|SetCurrentHealth (- (Variables|Health|GetCurrentHealth) DamageTaken))
      (CallFunction|BecomeInvulnerable true)
      (Components|Tick|SetComponentTickEnabled true)))
  (return))

(fn BecomeInvulnerable
  (params (IsInvulnerable :type Boolean))
  (LocalVariables|SetPreviousValue (Variables|Health|GetIsInvulnerable))
  (Variables|Health|SetIsInvulnerable IsInvulnerable)
  (if (!= (Variables|Health|GetIsInvulnerable) (LocalVariables|GetPreviousValue))
    (if (Variables|Health|GetIsInvulnerable)
      (Default|CallEDonBecomeInvulnerable)
      (else
        (Default|CallEDonLeaveInvulnerable)))))