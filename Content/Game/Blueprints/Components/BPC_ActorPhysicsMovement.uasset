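; Actor component that steers a physics-driven root primitive along its forward vector, with helpers for obstacle avoidance and impacts.
; ApplyMovement sets linear velocity from speed plus accumulated external forces, clearing them afterwards.
; ApplyRotation smoothly aligns the body to TargetDirection, then adds and clears quaternion-composed extra rotation.
; Helpers trace ahead, pick directions via cone rays, bank a scene component into turns, and compute impact speed and bounce direction.
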(event EventBeginPlay
  (bind _returnvalue (Components|GetOwner))
  (bind _asprimitive_component (Utilities|Casting|CastToPrimitiveComponent (Variables|/Script/Engine.Actor|GetRootComponent _returnvalue))
    (:then
      (Variables|Default|SetOwnRootPhysics _asprimitive_component)
      (Variables|Physics|Forces|Direction|SetTargetDirection (Math|Vector|GetForwardVector (Variables|Default|GetOwnRootPhysics))))
    (:CastFailed
      (Development|PrintText (Utilities|Text|FormatText "{n} not physiqued" (Utilities|GetDisplayName _returnvalue))))))

(fn SetForwardMovement
  (Variables|Physics|Forces|Movement|SetSelfForce (* (Variables|Physics|Forces|Speed|GetCurrentSpeed) (Math|Vector|GetForwardVector (Variables|Default|GetOwnRootPhysics))))
  (return))

(fn ApplyMovement
  (Movement|SetForwardMovement)
  (Physics|SetPhysicsLinearVelocity (Variables|Default|GetOwnRootPhysics) (+ (Variables|Physics|Forces|Movement|GetSelfForce) (Variables|Physics|Forces|Movement|GetOtherForces)) false "None")
  (Variables|Physics|Forces|Movement|SetOtherForces "0, 0, 0")
  (return))

(fn SetOtherForcesMovement
  (params (OtherForces :type Vector))
  (|SetBy-RefVar (Variables|Physics|Forces|Movement|GetOtherForces) (+ OtherForces (Variables|Physics|Forces|Movement|GetOtherForces))))

(fn ChangeDirectiontoRotation
  (bind (_currentrota _targetrota) (CallFunction|AlignVectors (Variables|Default|GetOwnRootPhysics) (Math|Vector|Normalize (Variables|Physics|Forces|Direction|GetTargetDirection))))
  (bind _returnvalue (CallFunction|AlignSmooth _currentrota _targetrota (Variables|Physics|Rotation|GetRotationRate)))
  (Variables|Physics|Rotation|SetTargetSelfRotation _returnvalue)
  (return))

(fn SetRandomDirection
  (params (ConeAngle :type Float%20%28double-precision%29) (Range :type Float%20%28double-precision%29) (RadiusToCover :type Integer))
  (bind _returnvalue (Components|GetOwner))
  (bind (_output _hasadirection) (CallFunction|GetOneDirectionfromSphereRadius 6 (Transformation|GetActorLocation _returnvalue) (Transformation|GetActorForwardVector _returnvalue) ConeAngle Range RadiusToCover "TraceTypeQuery1" "None" 2.0 "(R=0.000000,G=0.846483,B=1.000000,A=1.000000)"))
  (if _hasadirection
    (Variables|Physics|Forces|Direction|SetTargetDirection _output))
  (return))

(fn CanMovetoCurrentDirection
  (params (Range :type Float%20%28double-precision%29))
  (bind _returnvalue (Components|GetOwner))
  (bind _returnvalue_2 (Transformation|GetActorLocation _returnvalue))
  (bind _returnvalue_3 (Collision|LineTraceByChannel _returnvalue_2 (+ _returnvalue_2 (* Range (Transformation|GetActorForwardVector _returnvalue))) "TraceTypeQuery3" true 0 "None" true "(R=1.000000,G=0.545587,B=0.000000,A=1.000000)" "(R=0.000000,G=0.165606,B=1.000000,A=1.000000)" 0.0))
  (return (not _returnvalue_3)))

(fn SetOtherRotation
  (params (OtherRota :type Rotator))
  (bind _targetotherrotation (Variables|Physics|Rotation|GetTargetOtherRotation))
  (|SetBy-RefVar _targetotherrotation (Class|KismetMathLibrary|QuatRotator (* (Math|Conversions|ToQuaternion(Rotator) _targetotherrotation) (Class|KismetMathLibrary|QuatNormalized (Math|Conversions|ToQuaternion(Rotator) OtherRota) 0.0001))))
  (return))

(fn ApplyRotation
  (Rotation|ChangeDirectiontoRotation)
  (Transformation|SetWorldRotation (Variables|Default|GetOwnRootPhysics) (Variables|Physics|Rotation|GetTargetSelfRotation) false false)
  (Transformation|AddWorldRotation (Variables|Default|GetOwnRootPhysics) (Variables|Physics|Rotation|GetTargetOtherRotation) false false)
  (Variables|Physics|Rotation|SetTargetOtherRotation "0, 0, 0")
  (return))

(fn SetRollonSceneComp
  (params (Target :type Scene%20Component%20Object%20Reference%20%28by%20ref%29) (AngleMaxToRoll :type Float%20%28double-precision%29) (InterpSpeed :type Float%20%28single-precision%29))
  (bind _ownrootphysics (Variables|Default|GetOwnRootPhysics))
  (LocalVariables|SetAnglePower (Math|Float|NormalizetoRange (CallFunction|GetSideBetween2Vec (Math|Vector|GetForwardVector _ownrootphysics) (Math|Vector|Normalize (Variables|Physics|Forces|Direction|GetTargetDirection)) (Math|Vector|GetUpVector _ownrootphysics)) 0.0 0.1))
  (Transformation|SetRelativeRotation Target (Math|Interpolation|RInterpTo (Variables|/Script/Engine.SceneComponent|GetRelativeRotation Target) (Math|Rotator|MakeRotator (* (LocalVariables|GetAnglePower) AngleMaxToRoll) 0.0 0.0) (Utilities|Time|GetWorldDeltaSeconds) InterpSpeed) false false)
  (return))

(fn GetSpeed
  (return (Math|Vector|VectorLength (CallFunction|GetVelocity (Variables|Default|GetOwnRootPhysics)))))

(fn ChangeSpeedonImpact
  (params (ImpactNormalDirection :type Vector))
  (Variables|Physics|Forces|Speed|SetCurrentSpeed (+ (* (Variables|Physics|Forces|Speed|GetCurrentSpeed) (Math|Vector|DotProduct ImpactNormalDirection (Math|Vector|GetForwardVector (Variables|Default|GetOwnRootPhysics)))) (Variables|Physics|Forces|Speed|GetCurrentSpeed)))
  (return))

(fn GetBoundDirection
  (params (ImpactNormal :type Vector))
  (return (Math|Vector|Normalize (* (- (CallFunction|GetVelocity (Variables|Default|GetOwnRootPhysics)) (* (* (Math|Vector|DotProduct (Math|Vector|GetForwardVector (Variables|Default|GetOwnRootPhysics)) ImpactNormal) ImpactNormal) 2.0)) (Variables|Physics|Forces|Speed|GetCurrentSpeed)))))