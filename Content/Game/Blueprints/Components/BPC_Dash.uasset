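; BPC_Dash is an actor component that gives its owner a forward dash with a cooldown, driven through the owner's BPC_Movement component.
; A dash request enables Tick, which runs the cooldown and duration countdowns until the dash is ready again.
; Setters turn timer results into event dispatcher calls for state changes.
; While dashing, it repeatedly sends BPC_Movement a forward force scaled by remaining duration, so the push fades out.
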(event Custom|ED_OnDash_Event
  (if (Variables|Default|GetCanDash)
    (Variables|Cooldown|SetCurrentCooldown (Variables|Cooldown|GetMaxCooldown))
    (Components|Tick|SetComponentTickEnabled true)
    (Variables|Cooldown|SetCurrentDashDuration (Variables|Cooldown|GetMaxDashDuration))
    (Default|CallEDIsDashing)))

(event Custom|ED_DashReady_Event
  (Components|Tick|SetComponentTickEnabled false))

(event Custom|ED_OnDashActivated_Event)

(event Custom|ED_IsDashing_Event
  (bind _bpc_movement (Variables|Default|GetBPC_Movement))
  (bind _output_get (Variables|Param|SetDashForces (* (Math|Vector|GetForwardVector (Variables|/Game/Game/Blueprints/Components/BPC_Movement.BPC_Movement_C|GetRootOwner _bpc_movement)) (* (Variables|Param|GetDashPower) (Math|Float|NormalizetoRange (Variables|Cooldown|GetCurrentDashDuration) 0.0 (Variables|Cooldown|GetMaxDashDuration))))))
  (Default|SetOtherForces _bpc_movement _output_get))

(event Custom|ED_EndDash_Event)

(event EventBeginPlay
  ;[0 1 0.2971] Begin Play
  (EventDispatchers|BindEventtoEDonDash (EventDispatchers|CreateEvent :!event Custom|ED_OnDash_Event))
  (EventDispatchers|BindEventtoEDDashReady (EventDispatchers|CreateEvent :!event Custom|ED_DashReady_Event))
  (EventDispatchers|BindEventtoEDonDashActivated (EventDispatchers|CreateEvent :!event Custom|ED_OnDashActivated_Event))
  (EventDispatchers|BindEventtoEDIsDashing (EventDispatchers|CreateEvent :!event Custom|ED_IsDashing_Event))
  (EventDispatchers|BindEventtoEDEndDash (EventDispatchers|CreateEvent :!event Custom|ED_EndDash_Event))
  (Variables|Default|SetBPC_Movement (Actor|GetComponentbyClass (Components|GetOwner) "/Game/Game/Blueprints/Components/BPC_Movement.BPC_Movement_C")))

(event EventTick
  (params (DeltaSeconds :type Float%20%28single-precision%29))
  ;[1 0.19 0] Timers
  (CallFunction|SetCanDash (CallFunction|TimerNeg (Variables|Cooldown|GetCurrentCooldown) (Variables|Cooldown|GetMaxCooldown) 1.0 false))
  (CallFunction|SetinDash (not (CallFunction|TimerNeg (Variables|Cooldown|GetCurrentDashDuration) (Variables|Cooldown|GetMaxDashDuration) 1.0 false))))

(fn SetCanDash
  (params (OnValue :type Boolean))
  (LocalVariables|SetPreviousValue (Variables|Default|GetCanDash))
  (Variables|Default|SetCanDash OnValue)
  (if (!= (Variables|Default|GetCanDash) (LocalVariables|GetPreviousValue))
    (if (Variables|Default|GetCanDash)
      (Default|CallEDDashReady)
      (else
        (Default|CallEDonDashActivated)))
    (else
      (if (Variables|Default|GetCanDash)
        _
        (else
          _))
      (Development|PrintText (Utilities|Text|FormatText "Can Dash Is Already {x}" (Variables|Default|GetCanDash)) false true "(R=1.000000,G=0.413570,B=0.000000,A=1.000000)" 0.0))))

(fn SetinDash
  (params (OnValue :type Boolean))
  (LocalVariables|SetPreviousValue (Variables|Default|GetIsDashing))
  (Variables|Default|SetIsDashing OnValue)
  (if (!= (Variables|Default|GetIsDashing) (LocalVariables|GetPreviousValue))
    (if (Variables|Default|GetIsDashing)
      (Default|CallEDIsDashing)
      (else
        (Default|CallEDEndDash)))
    (elif (Variables|Default|GetIsDashing)
      (Default|CallEDIsDashing))))