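; Actor component that makes its owner bounce off other actors that also carry BPC_Bouncing.
; On BeginPlay it binds to the hit event of BPC_Movement's root component.
; On hit, it passes the normalized impulse to the other actor's ApplyBounce and fires a colliding dispatcher.
; ApplyBounce scales that direction by the receiver's own speed and BouncePower, then feeds it to BPC_Movement via SetOtherForces.
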(event Custom|ED_OnColliding_Event
  (Development|PrintText "Bouncing"))

(event Custom|BPC_Move_OnHit
  (params (HitComponent :type Primitive%20Component%20Object%20Reference) (OtherActor :type Actor%20Object%20Reference) (OtherComp :type Primitive%20Component%20Object%20Reference) (NormalImpulse :type Vector) (Hit :type Hit%20Result%20Structure%20%28by%20ref%29))
  (bind _returnvalue (Actor|GetComponentbyClass OtherActor "BPC_Bouncing_C"))
  (Utilities|IsValid _returnvalue
    (:Is%20Valid
      (CallFunction|ApplyBounce _returnvalue (Math|Vector|Normalize NormalImpulse))
      (Default|CallEDonColliding))))

(event EventBeginPlay
  (bind _output_get (Variables|Default|SetBPC_Move (Actor|GetComponentbyClass (Components|GetOwner) "/Game/Game/Blueprints/Components/BPC_Movement.BPC_Movement_C")))
  (Collision|BindEventtoOnComponentHit (Variables|/Game/Game/Blueprints/Components/BPC_Movement.BPC_Movement_C|GetRootOwner _output_get) (EventDispatchers|CreateEvent :!event Custom|BPC_Move_OnHit)))

(fn GetVelocityPower
  (return (* (Math|Vector|VectorLength (Transformation|GetComponentVelocity (Variables|/Game/Game/Blueprints/Components/BPC_Movement.BPC_Movement_C|GetRootOwner (Variables|Default|GetBPC_Move)))) (Variables|Default|GetBouncePower))))

(fn GetBouncePower
  (params (Normal :type Vector))
  (return (* Normal (CallFunction|GetVelocityPower))))

(fn ApplyBounce
  (params (NewParam :type Vector))
  (Default|SetOtherForces (Variables|Default|GetBPC_Move) (CallFunction|GetBouncePower NewParam)))