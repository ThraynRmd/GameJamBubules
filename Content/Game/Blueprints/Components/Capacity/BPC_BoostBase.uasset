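; Base actor component for boost capacities, providing shared add and remove lifecycle handling.
; On BeginPlay it binds handlers to its added and destroy-component event dispatchers.
; The added handler prints a debug message naming the target and this component, and the removed handler destroys the component.
; It applies no boost effect itself.
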(event Custom|ED_OnAdded_Event
  (params (Target :type Actor%20Object%20Reference))
  (Development|PrintText (Utilities|Text|FormatText "{x} add {y}" (Utilities|GetDisplayName Target) (Utilities|GetDisplayName self)) true true "(R=0.000000,G=1.000000,B=0.158184,A=1.000000)" 5.0))

(event Custom|ED_OnRemoved_Event
  (params (Target :type Actor%20Object%20Reference))
  (Components|DestroyComponent))

(event EventBeginPlay
  (EventDispatchers|BindEventtoEDonAdded (EventDispatchers|CreateEvent :!event Custom|ED_OnAdded_Event))
  (EventDispatchers|BindEventtoEDDestroyComponent (EventDispatchers|CreateEvent :!event Custom|ED_OnRemoved_Event)))