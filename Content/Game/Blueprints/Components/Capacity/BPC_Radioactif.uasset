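; BPC_Radioactif is a temporary, contagious radioactive actor component that spreads to players near its owner.
; On BeginPlay it activates the owner's sphere component, then after ten seconds deactivates it and destroys itself.
; Each tick it polls that sphere for overlapping BP_Player actors and calls AddBPCRadioactif on any lacking the component.
; A separate Destroy function re-activates the sphere rather than deactivating it before removing the component.
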(event EventBeginPlay
  (CallFunction|Init)
  (Utilities|FlowControl|Delay 1e+01)
  (Development|PrintString "Je vais me détruire")
  (Components|Activation|SetActive (Variables|Default|GetSphereCollision) false false)
  (Components|DestroyComponent))

(event EventTick
  (params (DeltaSeconds :type Float%20%28single-precision%29))
  (bind _spherecollision (Variables|Default|GetSphereCollision))
  (bind _overlappingactors (Collision|GetOverlappingActors _spherecollision "/Game/Game/Blueprints/BP_Player.BP_Player_C" :!class /Script/Engine.PrimitiveComponent))
  (if (not (Utilities|Array|IsEmpty _overlappingactors))
    (for _array_element _overlappingactors
      (Utilities|IsValid (Actor|GetComponentbyClass _array_element "BPC_Radioactif_C")
        (:Is%20Valid
          (Development|PrintString "SALUT J'EXISTE"))
        (:Is%20Not%20Valid
          (Game|AddComponentbyClass _array_element "BPC_Radioactif_C"))))))

(fn Init
  (bind _returnvalue (Components|GetOwner))
  (bind _returnvalue_2 (Actor|GetComponentbyClass _returnvalue "/Script/Engine.SphereComponent"))
  (Variables|Default|SetSphereCollision _returnvalue_2)
  (Components|Activation|SetActive _returnvalue_2 true true)
  (Development|PrintString "Salut ! Je suis le BPC_Radioactif et j'existe"))

(fn Destroy
  (Components|Activation|SetActive (Actor|GetComponentbyClass (Components|GetOwner) "/Script/Engine.SphereComponent") true true)
  (Components|DestroyComponent))