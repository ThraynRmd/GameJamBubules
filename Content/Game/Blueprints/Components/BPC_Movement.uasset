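; Movement component that drives its owner's physics-simulated root primitive from move and stop events.
; Move events set a target velocity from 2D direction and speed, then smoothly rotate the root toward that direction; stop events zero the target velocity.
; ApplyLocation, not called in this file, interpolates physics velocity toward the target and adds accumulated external forces, clearing them afterward.
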(event Custom|ED_OnMove_Event
  (params (Target :type Vector%202D%20Structure))
  (bind _output_get (Variables|Direction|SetTargetDirection (Math|Conversions|ToVector(Vector2D) Target)))
  (Variables|Forces|SetTargetVelocity (* _output_get (Variables|Speed|GetSpeed)))
  (HandleTransform|ApplyRotation))

(event Custom|ED_OnStopMove_Event
  (Development|PrintText "Stop")
  (Variables|Forces|SetTargetVelocity "0, 0, 0"))

(event EventBeginPlay
  (EventDispatchers|BindEventtoEDonMove (EventDispatchers|CreateEvent :!event Custom|ED_OnMove_Event))
  (EventDispatchers|BindEventtoEDonStopMove (EventDispatchers|CreateEvent :!event Custom|ED_OnStopMove_Event))
  (bind _asprimitive_component (Utilities|Casting|CastToPrimitiveComponent (Variables|/Script/Engine.Actor|GetRootComponent (Components|GetOwner)))
    (:then
      (bind _output_get (Variables|Default|SetRootOwner _asprimitive_component))
      (Physics|SetSimulatePhysics _output_get true))
    (:CastFailed
      (Development|PrintText "Root n'est pas primitif" true true "(R=1.000000,G=0.485079,B=0.000000,A=1.000000)" 5.0))))

(fn GetNextRotation
  (bind _rootowner (Variables|Default|GetRootOwner))
  (bind _targetdirection (Variables|Direction|GetTargetDirection))
  (bind _returnvalue (Math|Vector|Normalize _targetdirection))
  (bind (_currrota _targetrota) (CallFunction|AlignVector _rootowner _returnvalue))
  (return (CallFunction|AlignSmooth _currrota _targetrota (Variables|Direction|GetRotationRate))))

(fn ApplyLocation
  (bind _rootowner (Variables|Default|GetRootOwner))
  (Physics|SetPhysicsLinearVelocity _rootowner (+ (Math|Interpolation|VInterpTo (Transformation|GetComponentVelocity _rootowner) (Variables|Forces|GetTargetVelocity) (Utilities|Time|GetWorldDeltaSeconds) (Variables|Speed|GetInterpSpeed)) (Variables|Forces|GetOtherForces)) false "None")
  (Variables|Forces|SetOtherForces "0, 0, 0")
  (return))

(fn ApplyRotation
  (Transformation|SetWorldRotation (Variables|Default|GetRootOwner) (CallFunction|GetNextRotation) false false))

(fn SetSelfForce
  (Variables|Forces|SetTargetVelocity (* (Variables|Speed|GetSpeed) (Variables|Direction|GetTargetDirection)))
  (return))

(fn DecreaseForces
  (params (TargetToDecrease :type Vector%20%28by%20ref%29) (InterpSpeed :type Float%20%28single-precision%29))
  (|SetBy-RefVar TargetToDecrease (Math|Interpolation|VInterptoConstant TargetToDecrease "0, 0, 0" (Utilities|Time|GetWorldDeltaSeconds) InterpSpeed))
  (return))

(fn SetOtherForces
  (params (ForcesAdded :type Vector%20%28by%20ref%29))
  (bind _otherforces (Variables|Forces|GetOtherForces))
  (|SetBy-RefVar _otherforces (+ ForcesAdded _otherforces))
  (return))